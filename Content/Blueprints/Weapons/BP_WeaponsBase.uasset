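; Base weapon actor that handles in-hand versus inventory visibility and triggers attack animations.
; Inventory and in-hand events hide or show the root and its children.
; Attack calls PlayAttackAnim, which plays the AttackAnim montage on the skeletal mesh of the owning BP_CharacterBase.
; CommitAttackAnimNotify is an empty event, and the weapon has no active tick, overlap or BeginPlay logic.
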(event `WeaponInInventory`
  (`SceneComponent.SetVisibility` (`self.DefaultSceneRoot`) false true))

(event `WeaponInHand`
  (`SceneComponent.SetVisibility` (`self.DefaultSceneRoot`) true true))

(event `PlayAttackAnim`
  (`|PlayMontage` (`self.GetPawnSkeletalMesh`) (`self.AttackAnim`)))

(event `Attack`
  (`self.PlayAttackAnim`))

(event `CommitAttackAnimNotify`)

(fn `GetPawnSkeletalMesh`
  (returns (Mesh :type "SkeletalMeshComponent Object Reference"))
  (bind _asbp_character_base (cast `/Game/PlayerAssets/BP_CharacterBase` (`self.GetOwner`))
    (:`then`
      _)
    (:`CastFailed`
      _))
  (return (`Character.Mesh` _asbp_character_base)))

(fn `UserConstructionScript`)